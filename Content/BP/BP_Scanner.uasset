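; BP_Scanner is an actor that plays a visual scan pulse as an expanding sphere.
; DoScan runs on BeginPlay, unhides the actor and restarts a timeline that drives uniform actor scale and the Scanner_opacity material parameter on the sphere.
; The actor hides itself when the timeline finishes.
; Sphere collision is disabled at start and end, and the graph contains no detection logic.
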(event Custom|DoScan
  (Rendering|SetActorHiddenInGame false)
  (Collision|SetCollisionEnabled (Variables|Default|GetSphere) "NoCollision")
  (bind (_direction _scanner_expand_size _scanner_opacity) (Timeline|Timeline PlayFromStart)
    (:Update
      (Transformation|SetActorScale3D (Math|Conversions|ToVector(Float) _scanner_expand_size))
      (Rendering|Material|SetScalarParameterValueonMaterials (Variables|Default|GetSphere) "Scanner_opacity" _scanner_opacity))
    (:Finished
      (Collision|SetCollisionEnabled (Variables|Default|GetSphere) "NoCollision")
      (Rendering|SetActorHiddenInGame true))))

(event EventBeginPlay
  (CallFunction|DoScan))

(fn ConstructionScript)